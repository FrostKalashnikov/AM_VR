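; MasterItem_BP is a base VR collectible that awards the player a point when grabbed and then dissolves away.
; The first grab from its GrabComponent increments PointsNum on the VRPawn, disables collision and calls StartDissolve.
; StartDissolve removes the Plane and PLevelUpDetail components, puts a dynamic dissolve material on every static mesh slot and plays the pickup sound.
; A timeline drives the material's Amount and Boost parameters, then destroys the actor.
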(event `self.ReceiveBeginPlay`
  (bind _returnvalue (`KismetMaterialLibrary.CreateDynamicMaterialInstance` (`self.Material Dissolve`)))
  (set `self.MID_Dissolve` _returnvalue))

(event `self.GrabComponent.OnGrabbed`
  (`/Engine/EditorBlueprintResources/StandardMacros.DoOnce` false
    (:`Completed`
      (bind _asvrpawn (cast `/Game/VRTemplate/Blueprints/VRPawn` (`GameplayStatics.GetPlayerPawn` 0)))
      (`/Engine/EditorBlueprintResources/StandardMacros.IncrementInt` (`/Game/VRTemplate/Blueprints/VRPawn.PointsNum` _asvrpawn)
        (:`  `
          (`self.SetActorEnableCollision` false)
          (`self.Start Dissolve`))))))

(event `Start Dissolve`
  (bind _mid_dissolve (`self.MID_Dissolve`))
  (`ActorComponent.K2_DestroyComponent` (`self.Plane`))
  (`ActorComponent.K2_DestroyComponent` (`self.P_levelUp_Detail`))
  (for _array_element (`self.K2_GetComponentsByClass` "/Script/Engine.StaticMeshComponent")
    (`MeshComponent.SetOverlayMaterial` _array_element null)
    (for _index (range (+ (`PrimitiveComponent.GetNumMaterials` _array_element) 1))
      (`PrimitiveComponent.SetMaterial` _array_element _index (`self.MID_Dissolve`))))
  (`GameplayStatics.PlaySound2D` "/Game/CITY_PACK/VRTemplate/Blueprints/Arcelor_VR/Audio/PickUpSound_Cue.PickUpSound_Cue" 1.0 1.0 0.0 null null)
  (bind (_direction _amount _boost) (`Timeline|Timeline`)
    (:`Update`
      (`MaterialInstanceDynamic.SetScalarParameterValue` _mid_dissolve "Amount" _amount)
      (`MaterialInstanceDynamic.SetScalarParameterValue` _mid_dissolve "Boost" _boost))
    (:`Finished`
      (`self.K2_DestroyActor`))))

(fn `UserConstructionScript`)