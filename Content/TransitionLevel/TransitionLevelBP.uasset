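; Level transition manager that switches between streamed scenes behind a material-driven transition effect.
; SetTransitionScene picks a level and view target by index from the AllScenes map, with an optional target override, then plays a timeline driving the TransitionPC parameter collection.
; When the forward play finishes, it unloads the current level, blocking-loads the new one, switches the player's view target, reverses the timeline and calls CallRevertingTransition.
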(event `self.ReceiveBeginPlay`
  (`KismetMaterialLibrary.SetScalarParameterValue` "/Game/TransitionLevel/TransitionPC.TransitionPC" "Scalar" 3000000.0))

(event `Start Transition`
  (bind (_direction _scalar _alpha) (`Timeline|Transition` :!label _label)
    (:`Update`
      (`KismetMaterialLibrary.SetScalarParameterValue` "/Game/TransitionLevel/TransitionPC.TransitionPC" "Scalar" _scalar)
      (`KismetMaterialLibrary.SetScalarParameterValue` "/Game/TransitionLevel/TransitionPC.TransitionPC" "TransitionAlpha" _alpha))
    (:`Finished`
      (switch `ETimelineDirection` _direction
        (:`Forward`
          (`GameplayStatics.UnloadStreamLevelBySoftObjectPtr` (`self.Current Level`))
          (`GameplayStatics.LoadStreamLevelBySoftObjectPtr` (`self.New Level`) true true)
          (set `self.Current Level` (`self.New Level`))
          (`PlayerController.SetViewTargetWithBlend` (`GameplayStatics.GetPlayerController` 0) (`self.New View Target`) 0.0 "VTBlend_Linear" 0.0 false)
          (`self.Reverse Transition`)
          (`self.RevertingTransition`))))))

(event `Reverse Transition`
  (goto _label :!via `Reverse`))

(event `Set Transition Scene`
  (params (SceneID :type Integer) (`New View Target` :type "CineCameraActor Object Reference"))
  (bind _allscenes (`self.AllScenes`))
  (set `self.SceneID` SceneID)
  (bind _values (`BlueprintMapLibrary.Map_Values` _allscenes))
  (set `self.New View Target` (select `bool` (`KismetSystemLibrary.IsValid` `New View Target`) :`false` (`|GetArrayItem` _values (`self.SceneID`)) :`true` `New View Target`))
  (bind _keys (`BlueprintMapLibrary.Map_Keys` _allscenes))
  (set `self.New Level` (`|GetArrayItem` _keys (`self.SceneID`)))
  (`self.Start Transition`))

(fn `UserConstructionScript`)