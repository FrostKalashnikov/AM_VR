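; Master Blueprint actor that defines a spline flight path, apparently for Niagara particle birds to follow.
; The construction script sizes a collision sphere to the visibility radius and toggles its display.
; A single getter bundles the path settings, including spline length, loop state, probability, two-way travel, roaming boundary and end-of-path kill or flight type.
; Setters change probability, radius and disabled state, without resizing the sphere.
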(fn `DisablePath`
  (params (NewDisable :type Boolean))
  (set `self.DisabledPath` NewDisable))

(fn `GetPathInfo`
  (returns (Disabled :type Boolean) (PathLength :type "Float (double-precision)") (ClosedSpline :type Boolean) (KillParticles :type Boolean) (Boundary :type Boolean) (Probability :type "Float (double-precision)") (TwoDirections :type Boolean) (NewFlightType :type "/Game/BeefyBlackbirds/Blueprints/AI/ENiagaraFlightType Enum") (PathRadius :type "Float (double-precision)"))
  (return (`self.DisabledPath`) (`SplineComponent.GetSplineLength` (`self.Path`)) (`SplineComponent.IsClosedLoop` (`self.Path`)) (`self.KillParticlesWhenFinished`) (`self.RoamingParticleBoundary`) (`self.PathProbability`) (`self.AllowTwoDirections`) (`self.FinishedFlightType`) (`self.VisibilityRadius`)))

(fn `GetPathLength`
  (returns (Length :type "Float (double-precision)"))
  (return (`SplineComponent.GetSplineLength` (`self.Path`))))

(fn `SetPathProbability`
  (params (NewProbability :type "Float (double-precision)"))
  (set `self.PathProbability` NewProbability))

(fn `SetPathVisibilityRadius`
  (params (NewVisibilityRadius :type "Float (double-precision)"))
  (set `self.VisibilityRadius` NewVisibilityRadius))

(fn `UserConstructionScript`
  (`SphereComponent.SetSphereRadius` (`self.Collision`) (`self.VisibilityRadius`) true)
  (`SceneComponent.SetVisibility` (`self.Collision`) (`self.ShowCollision`) false))