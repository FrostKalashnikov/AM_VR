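; BP_Fridge is an interactive fridge prop with two swinging doors and a sliding BigDoor part.
; Any overlap with BoxColl toggles the icon and enables input for player 0, which is disabled on exit.
; Left click toggles the icon and drives three timelines, each playing or reversing based on its track value.
; The timelines set yaw on LeftDoor and RightDoor and Y location on BigDoor.
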(event `self.BoxColl.OnComponentBeginOverlap`
  (params (OverlappedComponent :type "PrimitiveComponent Object Reference") (OtherActor :type "Actor Object Reference") (OtherComp :type "PrimitiveComponent Object Reference") (OtherBodyIndex :type Integer) (bFromSweep :type Boolean) (SweepResult :type "HitResult Structure (by ref)"))
  (`self.EnableInput` (`GameplayStatics.GetPlayerController` 0))
  (`SceneComponent.ToggleVisibility` (`self.icon`) false :!label _label))

(event `self.BoxColl.OnComponentEndOverlap`
  (params (OverlappedComponent :type "PrimitiveComponent Object Reference") (OtherActor :type "Actor Object Reference") (OtherComp :type "PrimitiveComponent Object Reference") (OtherBodyIndex :type Integer))
  (`self.DisableInput` (`GameplayStatics.GetPlayerController` 0))
  (goto _label))

(event `Key|LeftMouseButton`
  (params (Key :type "Key Structure"))
  (:`Pressed`
    (`SceneComponent.ToggleVisibility` (`self.icon`) false)))

(event `Key|LeftMouseButton`
  (params (Key :type "Key Structure"))
  (:`Pressed`
    (if (< (stale _newtrack_0) 1.0)
      (bind (_direction _newtrack_0) (`Timeline|Timeline_2` :!label _label_2)
        (:`Update`
          (`SceneComponent.K2_SetRelativeRotation` (`self.LeftDoor`) (`KismetMathLibrary.MakeRotator` 0.0 0.0 _newtrack_0) false false)))
      (else
        (goto _label_2 :!via `Reverse`)))))

(event `Key|LeftMouseButton`
  (params (Key :type "Key Structure"))
  (:`Pressed`
    (if (> (stale _newtrack_0) -1.0)
      (bind (_direction _newtrack_0) (`Timeline|Timeline_3` :!label _label_3)
        (:`Update`
          (`SceneComponent.K2_SetRelativeRotation` (`self.RightDoor`) (`KismetMathLibrary.MakeRotator` 0.0 0.0 _newtrack_0) false false)))
      (else
        (goto _label_3 :!via `Reverse`)))))

(event `Key|LeftMouseButton`
  (params (Key :type "Key Structure"))
  (:`Pressed`
    (if (> 1.0 (stale _newtrack_0))
      (bind (_direction _newtrack_0) (`Timeline|Timeline_0` :!label _label_4)
        (:`Update`
          (`SceneComponent.K2_SetRelativeTransform` (`self.BigDoor`) (`KismetMathLibrary.MakeTransform` (`KismetMathLibrary.MakeVector` 0.0 _newtrack_0)) false false)))
      (else
        (goto _label_4 :!via `Reverse`)))))

(fn `UserConstructionScript`)